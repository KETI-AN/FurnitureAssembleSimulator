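; BP_AssembleFurniture drives automated, repeatable furniture assembly runs through the MainHUD held by FAS_GameMode.
; Tick waits until FAS_GameState is ready with IsStopAssemble set, then clears that flag to trigger one run.
; Each run loads and sets PDDL, mix-drops parts, starts physics, sets cargo and starts assembly, spaced by fixed Delays.
; It then prints and increments a repeat counter; a shorter sequence without PDDL steps is left unconnected.
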(event EventBeginPlay
  (bind _asfas_game_state (Utilities|Casting|CastToFAS_GameState (Game|GetGameState)))
  (Variables|Default|SetFAS_GameState _asfas_game_state)
  (bind _asfas_game_mode (Utilities|Casting|CastToFAS_GameMode (Game|GetGameMode)))
  (Variables|Default|SetFAS_GameMode _asfas_game_mode))

(event EventTick
  (params (DeltaSeconds :type Float%20%28single-precision%29))
  (bind _fas_gamestate (Variables|Default|GetFAS_GameState))
  (bind _fas_gamemode (Variables|Default|GetFAS_GameMode))
  (bind _mainhud (Variables|/Game/FAS_GameMode.FAS_GameMode_C|GetMainHUD _fas_gamemode))
  (if (and (Variables|/Game/FAS_GameState.FAS_GameState_C|GetisReadyForStart _fas_gamestate) (Variables|/Game/FAS_GameState.FAS_GameState_C|GetisStopAssemble _fas_gamestate))
    (Variables|/Game/FAS_GameState.FAS_GameState_C|SetisStopAssemble (Variables|Default|GetFAS_GameState) false)
    (Default|LoadPDDL _mainhud)
    (Utilities|FlowControl|Delay 4.0)
    (Default|SetPDDL _mainhud)
    (Utilities|FlowControl|Delay 4.0)
    (Default|MixDropFurnitureParts _mainhud)
    (Utilities|FlowControl|Delay 0.5)
    (Default|GoPhysic _mainhud)
    (Utilities|FlowControl|Delay 3.0)
    (Default|SetFurnitureCargoforAssemble _mainhud)
    (Default|FurnitureAssembleStart _mainhud)
    (Utilities|FlowControl|Delay 5.0)
    (CallFunction|DisplayRepeatCount)))

(fn ConstructionScript)

(fn DisplayRepeatCount
  (Development|PrintString (Utilities|String|Append "[Furniture Assemble Repeat] Current number of Counter is " (Utilities|String|ToString(Integer) (Variables|Default|GetnumCount))) true true "(R=0.013732,G=1.000000,B=0.000000,A=1.000000)" 1e+02)
  (Math|Integer|IncrementInt (Variables|Default|GetnumCount)))