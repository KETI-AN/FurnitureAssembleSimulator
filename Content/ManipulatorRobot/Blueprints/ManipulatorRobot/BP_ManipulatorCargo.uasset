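; Cargo actor for a manipulator robot, with events that flag it as carried and enable physics and gravity.
; The construction script applies CargoMesh, sizes the bound box from mesh bounds and passes scaled extents and roll to an optional Target's box.
; GetBoundBox returns scaled dimensions, with X and Y overridable when AutoBounds is off.
; BeginPlay clears the carried flag and prints a warning when no mesh is set.
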(event Custom|EnablePhysic
  (bind _staticmeshcargo (Variables|Default|GetStaticMeshCargo))
  (Physics|SetEnableGravity _staticmeshcargo true)
  (Physics|SetSimulatePhysics _staticmeshcargo true))

(event Custom|SetCargoCarried
  (Variables|Default|Setiscarried true))

(event EventBeginPlay
  (Variables|Default|Setiscarried false)
  (Utilities|IsValid (Variables|/Script/Engine.StaticMeshComponent|GetStaticMesh (Variables|Default|GetStaticMeshCargo))
    (:Is%20Not%20Valid
      (Development|PrintString (Utilities|String|Append "Mesh for cargo: " (Utilities|GetDisplayName self) " not set!") true true "(R=1.000000,G=0.892819,B=0.000000,A=1.000000)" 5.0))))

(event Collision|EventActorBeginOverlap
  (params (OtherActor :type Actor%20Object%20Reference)))

(fn ConstructionScript
  (bind _cargomesh (Variables|Cargo|GetCargoMesh))
  (Components|StaticMesh|SetStaticMesh (Variables|Default|GetStaticMeshCargo) _cargomesh)
  (Utilities|IsValid _cargomesh
    (:Is%20Valid
      (bind _output_get (Variables|Default|SetCargoBounds (.BoxExtent (Math|BoxSphereBounds|BreakBoxSphereBounds (StaticMesh|GetBounds _cargomesh)))))
      (if (Variables|Cargo|GetAutoBounds)
        (Variables|Cargo|SetBoundX (.X (Math|Vector|BreakVector _output_get)))
        (Variables|Cargo|SetBoundY (.Y (Math|Vector|BreakVector _output_get)))
        (Variables|Cargo|SetBoundZ (.Z (Math|Vector|BreakVector _output_get)))
        (else
          (Variables|Cargo|SetBoundZ (.Z (Math|Vector|BreakVector _output_get)))
          (LocalVariables|Setbounds (Math|Vector|MakeVector (Variables|Cargo|GetBoundX) (Variables|Cargo|GetBoundY) (.Z (Math|Vector|BreakVector _output_get))))))
      (Components|Box|SetBoxExtent (Variables|Default|GetCargoBoundBox) (Variables|Default|GetCargoBounds) true)
      (Utilities|IsValid (Variables|Cargo|GetTarget)
        (:Is%20Valid
          (CallFunction|UpdateTarget))))))

(fn GetBoundBox
  (return (* (Math|Vector|MakeVector (Variables|Cargo|GetBoundX) (Variables|Cargo|GetBoundY) (Variables|Cargo|GetBoundZ)) (.Scale (Math|Transform|BreakTransform (Transformation|GetActorTransform))))))

(fn SetCargoMesh
  (params (Mesh :type Static%20Mesh%20Object%20Reference))
  (Components|StaticMesh|SetStaticMesh (Variables|Default|GetStaticMeshCargo) Mesh))

(fn UpdateTarget
  (Components|Box|SetBoxExtent (Variables|/Game/ManipulatorRobot/Blueprints/ManipulatorRobot/BP_ManipulatorTarget.BP_ManipulatorTarget_C|GetTargetBoundBox (Variables|Cargo|GetTarget)) (* (Variables|Default|GetCargoBounds) (.Scale (Math|Transform|BreakTransform (Transformation|GetActorTransform)))) true)
  (Transformation|SetRelativeRotation (Variables|/Game/ManipulatorRobot/Blueprints/ManipulatorRobot/BP_ManipulatorTarget.BP_ManipulatorTarget_C|GetTargetBoundBox (Variables|Cargo|GetTarget)) (Math|Rotator|MakeRotator (Variables|Cargo|GetTargetRoll) 0.0 0.0) false false))