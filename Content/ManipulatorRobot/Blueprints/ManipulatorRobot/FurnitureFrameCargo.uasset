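; Cargo actor for a manipulator robot (furniture frame) that sizes itself from its mesh and configures its linked Target drop volume to match.
; On construction and BeginPlay it derives a bound box from the mesh bounds or manual X/Y values, offsetting it for off-centre pivots.
; The Target's box receives the scaled extent, roll and offset.
; Events flag the cargo as carried or enable gravity and physics.
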(event Custom|EnablePhysic
  (bind _staticmeshcargo (Variables|Default|GetStaticMeshCargo))
  (Physics|SetEnableGravity _staticmeshcargo true)
  (Physics|SetSimulatePhysics _staticmeshcargo true))

(event Custom|SetCargoCarried
  (Variables|Default|Setiscarried true))

(event EventBeginPlay
  (Variables|Default|Setiscarried false)
  (Utilities|IsValid (Variables|/Script/Engine.StaticMeshComponent|GetStaticMesh (Variables|Default|GetStaticMeshCargo))
    (:Is%20Valid
      (CallFunction|SetTargetRollRotation)
      (CallFunction|SetCargoBoundBoxLocation)
      (CallFunction|SetCargoBoundBoxExtent)
      (CallFunction|UpdateTarget))
    (:Is%20Not%20Valid
      (Development|PrintString (Utilities|String|Append "Mesh for cargo: " (Utilities|GetDisplayName self) " not set!") true true "(R=1.000000,G=0.892819,B=0.000000,A=1.000000)" 5.0))))

(event Collision|EventActorBeginOverlap
  (params (OtherActor :type Actor%20Object%20Reference)))

(fn ConstructionScript
  (bind _cargomesh (Variables|Cargo|GetCargoMesh))
  ;[1 1 1] Set Static Mesh
  (Components|StaticMesh|SetStaticMesh (Variables|Default|GetStaticMeshCargo) _cargomesh)
  (Utilities|IsValid _cargomesh
    (:Is%20Valid
      (CallFunction|SetTargetRollRotation)
      (CallFunction|SetCargoBoundBoxLocation)
      (CallFunction|SetCargoBoundBoxExtent)
      (CallFunction|UpdateTarget))
    (:Is%20Not%20Valid
      (Development|PrintString (Utilities|String|Append "Staric Mesh: " (Utilities|GetDisplayName _cargomesh) " is not valid!")))))

(fn GetBoundBox
  (return (* (Math|Vector|MakeVector (Variables|Cargo|GetBoundX) (Variables|Cargo|GetBoundY) (Variables|Cargo|GetBoundZ)) (.Scale (Math|Transform|BreakTransform (Transformation|GetActorTransform))))))

(fn SetCargoMesh
  (params (Mesh :type Static%20Mesh%20Object%20Reference))
  (Components|StaticMesh|SetStaticMesh (Variables|Default|GetStaticMeshCargo) Mesh))

(fn UpdateTarget
  (bind _target (Variables|Cargo|GetTarget))
  (bind _target_2 (Variables|Cargo|GetTarget))
  (bind _targetboundbox (Variables|/Game/ManipulatorRobot/Blueprints/ManipulatorRobot/FurnitureCargoTarget.FurnitureCargoTarget_C|GetTargetBoundBox _target_2))
  (Utilities|IsValid _target
    (:Is%20Valid
      (Components|Box|SetBoxExtent (Variables|/Game/ManipulatorRobot/Blueprints/ManipulatorRobot/FurnitureCargoTarget.FurnitureCargoTarget_C|GetTargetBoundBox _target) (* (Variables|Default|GetCargoBounds) (.Scale (Math|Transform|BreakTransform (Transformation|GetActorTransform)))) true)
      (Transformation|SetRelativeRotation _targetboundbox (Math|Rotator|MakeRotator (Variables|Cargo|GetTargetRoll) 0.0 0.0) false false)
      (if (not (Variables|Default|GetisOriginZero))
        (Transformation|SetRelativeLocation _targetboundbox (+ (Transformation|GetActorLocation _target_2) (Variables|Default|GetCargoOrigin)) false false)))
    (:Is%20Not%20Valid
      (Development|PrintString "Cargo's Target is Not Vaild."))))

(fn SetCargoBoundBoxLocation
  (bind _cargomesh (Variables|Cargo|GetCargoMesh))
  (bind _target (Variables|Cargo|GetTarget))
  (bind _returnvalue (StaticMesh|GetBounds _cargomesh))
  (bind _returnvalue_2 (Transformation|GetActorLocation _target))
  (bind (_origin _boxextent) (Math|BoxSphereBounds|BreakBoxSphereBounds _returnvalue))
  (bind (_x _y) (Math|Vector|BreakVector _returnvalue_2))
  ;[1 1 1] Check Cargo Pivot is Zero and Set Cargo Bound Box Location to Cargo Center Point
  (Variables|Default|SetCargoBounds _boxextent)
  (bind _output_get (Variables|Default|SetCargoOrigin _origin))
  (if (and (== (.X (Math|Vector|BreakVector _output_get)) 0.0) (== (.Y (Math|Vector|BreakVector _output_get)) 0.0))
    (Variables|Default|SetisOriginZero true)
    (else
      (Variables|Default|SetisOriginZero false)
      (Transformation|SetRelativeLocation (Variables|Default|GetCargoBoundBox) _output_get false false)))
  (Variables|Default|SetMovingYvalue (+ _y (.Y (Math|Vector|BreakVector _output_get))))
  (Variables|Default|SetMovingXvalue (+ _x (.X (Math|Vector|BreakVector _output_get)))))

(fn SetTargetRollRotation
  ;[1 1 1] Set Changed Target Roll Rotation to Target Bound Box
  (Transformation|SetRelativeRotation (Variables|/Game/ManipulatorRobot/Blueprints/ManipulatorRobot/FurnitureCargoTarget.FurnitureCargoTarget_C|GetTargetBoundBox (Variables|Cargo|GetTarget)) (Math|Rotator|MakeRotator (Variables|Cargo|GetTargetRoll) 0.0 0.0) false false))

(fn SetCargoBoundBoxExtent
  (bind _cargobounds (Variables|Default|GetCargoBounds))
  (bind _cargoboundbox (Variables|Default|GetCargoBoundBox))
  (bind (_x _y _z) (Math|Vector|BreakVector _cargobounds))
  ;[1 1 1] Set Cargo Bounds Box
  (if (Variables|Cargo|GetAutoBounds)
    (Variables|Cargo|SetBoundX _x)
    (Variables|Cargo|SetBoundY _y)
    (Variables|Cargo|SetBoundZ _z)
    (Components|Box|SetBoxExtent _cargoboundbox (Variables|Default|GetCargoBounds) true)
    (else
      (bind _output_get (Variables|Cargo|SetBoundZ _z))
      (bind _output_get_2 (Variables|Default|SetManualBounds (Math|Vector|MakeVector (Variables|Cargo|GetBoundX) (Variables|Cargo|GetBoundY) _output_get)))
      (Components|Box|SetBoxExtent _cargoboundbox _output_get_2 true))))