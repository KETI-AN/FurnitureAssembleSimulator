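; Chair Part 4 actor in a keyboard-driven assembly demo, starting at a fixed pose and joining Chair Part 5.
; G starts a per-Tick slide along +Y until a component hit stops it and enables gravity.
; F and H snap its Y position to simulate failed or successful assembly.
; Hits and F pulse the FAS_GameMode collision flag for a few seconds, while H pulses the assemble flag.
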(event OnComponentHit(StaticMeshComponent)
  (params (HitComponent :type Primitive%20Component%20Object%20Reference) (OtherActor :type Actor%20Object%20Reference) (OtherComp :type Primitive%20Component%20Object%20Reference) (NormalImpulse :type Vector :default "0, 0, 0") (Hit :type Hit%20Result%20Structure%20%28by%20ref%29))
  (bind _newgamemode (Variables|Default|GetNewGameMode))
  ;[1 1 1] Hit Chair Part 5 and Set Gravity
  (Variables|Default|SetbIsMoving false)
  (Physics|SetEnableGravity (Variables|Debug|GetStaticMeshComponent) true)
  (Variables|/Game/FAS_GameMode.FAS_GameMode_C|SetIsHitCollision _newgamemode true)
  (Utilities|FlowControl|Delay 5.0)
  (Variables|/Game/FAS_GameMode.FAS_GameMode_C|SetIsHitCollision _newgamemode false))

(event EventBeginPlay
  ;[1 1 1] Set Initial Transform
  (Input|EnableInput (Game|GetPlayerController 0))
  (Transformation|SetActorTransform (Math|Transform|MakeTransform "-44.000000,-100.000000,135.850006" "0.000000,90.000000,-82.000000") true)
  (Development|PrintString "[INIT] Chair Part 4 Transform is initialized." true true "(R=0.000000,G=1.000000,B=0.000000,A=1.000000)")
  (bind _asfas_game_mode (Utilities|Casting|CastToFAS_GameMode (Game|GetGameMode)))
  (Variables|Default|SetNewGameMode _asfas_game_mode))

(event EventTick
  (params (DeltaSeconds :type Float%20%28single-precision%29))
  (bind _returnvalue (Transformation|GetActorLocation))
  (bind (_x _y _z) (Math|Vector|BreakVector _returnvalue))
  ;[1 1 1] Move Chair Part 4 to Chair Part 5
  (if (Variables|Default|GetbIsMoving)
    (Transformation|SetActorTransform (Math|Transform|MakeTransform (Math|Vector|MakeVector _x (+ _y 0.5) _z) (Transformation|GetActorRotation)))))

(event Input|KeyboardEvents|G
  (params (Key :type Key%20Structure :default "None"))
  ;[1 1 1] Set Moving Part Key Event
  (:Pressed
    (Development|PrintString "[MOVE] Chair Part 4 is moving to Chair Part 5" true true "(R=0.000000,G=0.000000,B=1.000000,A=1.000000)")
    (if (not (Variables|Default|GetbIsMoving))
      (Variables|Default|SetbIsMoving true))))

(event Input|KeyboardEvents|F
  (params (Key :type Key%20Structure :default "None"))
  (bind _returnvalue (Transformation|GetActorLocation))
  (bind _newgamemode (Variables|Default|GetNewGameMode))
  (bind (_x _y _z) (Math|Vector|BreakVector _returnvalue))
  ;[1 1 1] Failed Assemble Chair Part 4 and 5 Key Event
  (:Pressed
    (Development|PrintString "[ASSEMBLE FAIL] Chair Part 4 is assembled to Chair Part 5" true true "(R=1.000000,G=0.185686,B=0.845691,A=1.000000)")
    (Transformation|SetActorTransform (Math|Transform|MakeTransform (Math|Vector|MakeVector _x 0.0 _z) (Transformation|GetActorRotation)) true)
    (Variables|/Game/FAS_GameMode.FAS_GameMode_C|SetIsHitCollision _newgamemode true)
    (Utilities|FlowControl|Delay 5.0)
    (Variables|/Game/FAS_GameMode.FAS_GameMode_C|SetIsHitCollision _newgamemode false)))

(event Input|KeyboardEvents|H
  (params (Key :type Key%20Structure :default "None"))
  (bind _returnvalue (Transformation|GetActorLocation))
  (bind _newgamemode (Variables|Default|GetNewGameMode))
  (bind (_x _y _z) (Math|Vector|BreakVector _returnvalue))
  ;[1 1 1] Success Assemble Chair Part 4 and 5 Key Event
  (:Pressed
    (Development|PrintString "[ASSEMBLE OK] Chair Part 4 is assembled to Chair Part 5" true true "(R=1.000000,G=1.000000,B=0.000000,A=1.000000)")
    (Transformation|SetActorTransform (Math|Transform|MakeTransform (Math|Vector|MakeVector _x -18.300001 _z) (Transformation|GetActorRotation)) true true)
    (Variables|/Game/FAS_GameMode.FAS_GameMode_C|SetIsAssemble _newgamemode true)
    (Utilities|FlowControl|Delay 5.0)
    (Variables|/Game/FAS_GameMode.FAS_GameMode_C|SetIsAssemble _newgamemode false)))

(fn ConstructionScript)